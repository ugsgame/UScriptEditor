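; BP_PlayerCharacter is the player character Blueprint, set up as a thin shell around an attached Script object.
; GetModuleContext exposes the script's path, source code and bytecode, and GetModuleName returns its dot path as the module name.
; The only event logic is a Dummy event that plays the ZoomInOut timeline, and the construction script is empty.
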(event `Dummy`
  (`Timeline|ZoomInOut`))

(fn `GetModuleContext`
  (returns (Path :type String) (SourceCode :type String) (ByteCode :type "Array of Byte"))
  (bind _script (`self.Script`))
  (return (`ScriptDataAsset.GetPath` _script) (`ScriptDataAsset.GetSourceCode` _script) (`ScriptDataAsset.GetByteCode` _script)))

(fn `GetModuleName`
  (returns (ReturnValue :type String))
  (return (`ScriptDataAsset.GetDotPath` (`self.Script`))))

(fn `UserConstructionScript`)